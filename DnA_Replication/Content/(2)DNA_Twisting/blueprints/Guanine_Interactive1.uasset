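; Interactive guanine actor for the DNA twisting content, with looping movement and a toggleable highlight.
; On BeginPlay, two timelines hand off to each other on finish, one forward and one reversed, each driving the Guanine component's relative location.
; Tick polls the player controller for the 3 key, and a looping MultiGate alternates the material between a Fresnel glow and orange on each press.
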(event `self.ReceiveBeginPlay`
  (bind (_direction _newtrack_0) (`Timeline|Timeline` :!label _label)
    (:`Update`
      (`SceneComponent.K2_SetRelativeLocation` (`self.Guanine`) _newtrack_0 false false))
    (:`Finished`
      (bind (_direction_2 _newtrack_0_2) (`Timeline|Timeline_0` :!via `Reverse`)
        (:`Update`
          (`SceneComponent.K2_SetRelativeLocation` (`self.Guanine`) _newtrack_0_2 false false))
        (:`Finished`
          (goto _label :!via `PlayFromStart`))))))

(event `self.ReceiveTick`
  (params (DeltaSeconds :type "Float (single-precision)"))
  (bind _guanine (`self.Guanine`))
  (bind _returnvalue (`InputDeviceLibrary.GetPlayerControllerFromInputDevice` (struct)))
  (if (`PlayerController.WasInputKeyJustPressed` _returnvalue "Three")
    (`|MultiGate` false true
      (:`Out 0`
        (`PrimitiveComponent.SetMaterial` _guanine 0 "/Game/(2)DNA_Twisting/material_test/Fresnel_Mat_Glow.Fresnel_Mat_Glow"))
      (:`Out 1`
        (`PrimitiveComponent.SetMaterial` _guanine 0 "/Game/Level_9/subs_orange_inst.subs_orange_inst")))))

(fn `UserConstructionScript`)